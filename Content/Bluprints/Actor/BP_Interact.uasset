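; BP_Interact is an interactable actor that lets the player interact with it, intended to show a "press E to interact" prompt when nearby.
; Its Box collision detects actors tagged "player" entering or leaving, then casts player pawn 0 to BP_L2Player.
; On entry it registers itself through ChangeCurInteractActor, and on exit it calls the same function with no actor to clear it.
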(event OnComponentBeginOverlap(Box)
  (params (OverlappedComponent :type Primitive%20Component%20Object%20Reference) (OtherActor :type Actor%20Object%20Reference) (OtherComp :type Primitive%20Component%20Object%20Reference) (OtherBodyIndex :type Integer) (bFromSweep :type Boolean) (SweepResult :type Hit%20Result%20Structure%20%28by%20ref%29))
  ;[0.15 0.15 0.15 0.5] 通过碰撞检测显示“按E交互”
  (if (Actor|ActorHasTag OtherActor "player")
    (bind _asbp_l2player (Utilities|Casting|CastToBP_L2Player (Game|Player|GetPlayerPawn 0)))
    (Default|ChangeCurInteractActor _asbp_l2player self)))

(event OnComponentEndOverlap(Box)
  (params (OverlappedComponent :type Primitive%20Component%20Object%20Reference) (OtherActor :type Actor%20Object%20Reference) (OtherComp :type Primitive%20Component%20Object%20Reference) (OtherBodyIndex :type Integer))
  ;[0.15 0.15 0.15 0.5] 通过碰撞检测显示“按E交互”
  (if (Actor|ActorHasTag OtherActor "player")
    (bind _asbp_l2player (Utilities|Casting|CastToBP_L2Player (Game|Player|GetPlayerPawn 0)))
    (Default|ChangeCurInteractActor _asbp_l2player)))

(event EventBeginPlay)

(fn ConstructionScript)