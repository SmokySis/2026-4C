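; BP_LingGan is an interaction trigger actor that shows a WBP_E widget, likely a key prompt, when the first-person character overlaps it.
; On begin overlap with BP_Character_FP, it registers itself as the character's CurCamera, passes its UI reference to the character, and adds the widget to the viewport.
; End overlap removes the widget without checking which actor left or clearing the character's references.
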(event Collision|EventActorEndOverlap
  (params (OtherActor :type Actor%20Object%20Reference))
  (Widget|RemovefromParent (Variables|Default|GetUI_E)))

(event Collision|EventActorBeginOverlap
  (params (OtherActor :type Actor%20Object%20Reference))
  (bind _returnvalue (Actor|GetActorOfClass "/Game/Bluprints/Characters/Player/BP_Character_FP.BP_Character_FP_C"))
  (if (== _returnvalue OtherActor)
    (Utilities|FlowControl|Sequence
      (:then_0
        (Variables|/Game/Bluprints/Characters/Player/BP_Character.BP_Character_C|SetCurCamera _returnvalue self))
      (:then_2
        (Variables|/Game/Bluprints/Characters/Player/BP_Character.BP_Character_C|SetUI _returnvalue (Variables|Default|GetUI)))
      (:then_3
        (bind _returnvalue_2 (UserInterface|CreateWidget "/Game/UI/WBP_E.WBP_E_C"))
        (bind _output_get (Variables|Default|SetUI_E _returnvalue_2))
        (UserInterface|Viewport|AddtoViewport _output_get 0)))))

(fn ConstructionScript)