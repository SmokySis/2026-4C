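; BP_NPC is an NPC actor meant to show dialogue when interacted with.
; Its Interact event, commented as an interface call, passes the UniqueID variable to ShowDialogueByID.
; That function only prints the ID as a string, with no dialogue lookup or UI.
; The Box overlap event is empty, and Tick and actor overlap are disabled.
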(event OnComponentBeginOverlap(Box)
  (params (OverlappedComponent :type Primitive%20Component%20Object%20Reference) (OtherActor :type Actor%20Object%20Reference) (OtherComp :type Primitive%20Component%20Object%20Reference) (OtherBodyIndex :type Integer) (bFromSweep :type Boolean) (SweepResult :type Hit%20Result%20Structure%20%28by%20ref%29)))

(event Collision|EventActorBeginOverlap
  (params (OtherActor :type Actor%20Object%20Reference))
  (|CallParentFunction OtherActor) ; 此节点被禁用，将不会被调用。\n从引脚连出引线来编译功能。
)

(event EventInteract
  ;[0.15 0.15 0.15 0.5] 通过接口显示对话
  (CallFunction|ShowDialoguebyID (Variables|Default|GetUniqueID self)))

(event EventTick
  (params (DeltaSeconds :type Float%20%28single-precision%29))
  (|CallParentFunction DeltaSeconds) ; 此节点被禁用，将不会被调用。\n从引脚连出引线来编译功能。
)

(event EventBeginPlay
  (|CallParentFunction))

(fn ConstructionScript
  (|CallParentFunction))

(fn ShowDialoguebyID
  (params (UniqueID :type String))
  (Development|PrintString UniqueID))