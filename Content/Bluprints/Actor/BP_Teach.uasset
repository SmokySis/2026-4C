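; BP_Teach is an interactable actor that appears intended to show a tutorial entry identified by its UniqueID.
; A Box overlap with an actor tagged "player" toggles an outline by setting or clearing the M_PP_Outline overlay material on its StaticMesh.
; The Interact event passes UniqueID to ShowTeachByID, whose body is empty in this Blueprint.
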(event OnComponentBeginOverlap(Box)
  (params (OverlappedComponent :type Primitive%20Component%20Object%20Reference) (OtherActor :type Actor%20Object%20Reference) (OtherComp :type Primitive%20Component%20Object%20Reference) (OtherBodyIndex :type Integer) (bFromSweep :type Boolean) (SweepResult :type Hit%20Result%20Structure%20%28by%20ref%29))
  (if (Actor|ActorHasTag OtherActor "player")
    (CallFunction|SetOutline true)))

(event OnComponentEndOverlap(Box)
  (params (OverlappedComponent :type Primitive%20Component%20Object%20Reference) (OtherActor :type Actor%20Object%20Reference) (OtherComp :type Primitive%20Component%20Object%20Reference) (OtherBodyIndex :type Integer))
  (if (Actor|ActorHasTag OtherActor "player")
    (CallFunction|SetOutline false)))

(event Collision|EventActorBeginOverlap
  (params (OtherActor :type Actor%20Object%20Reference))
  (|CallParentFunction OtherActor) ; 此节点被禁用，将不会被调用。\n从引脚连出引线来编译功能。
)

(event EventTick
  (params (DeltaSeconds :type Float%20%28single-precision%29))
  (|CallParentFunction DeltaSeconds) ; 此节点被禁用，将不会被调用。\n从引脚连出引线来编译功能。
)

(event EventInteract
  (CallFunction|ShowTeachbyID (Variables|Default|GetUniqueID self)))

(fn ConstructionScript
  (|CallParentFunction))

(fn SetOutline
  (params (IsOn? :type Boolean))
  (bind _staticmesh (Variables|Default|GetStaticMesh))
  (if IsOn?
    (Rendering|Material|SetOverlayMaterial _staticmesh "/Game/Materials/M_PP_Outline.M_PP_Outline" :!class /Script/Engine.MeshComponent)
    (else
      (Rendering|Material|SetOverlayMaterial _staticmesh 0 :!class /Script/Engine.MeshComponent))))

(fn ShowTeachbyID
  (params (UniqueID :type String)))