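; BP_Controller is a player controller that handles first-person movement and look, plus a debug toggle for a riddle screen.
; BeginPlay adds the IMC_FP Enhanced Input context.
; IA_Move moves the pawn along its yaw-based forward and right vectors, while IA_Look feeds yaw and pitch.
; Debug key M alternately creates and removes WBP_Riddle_1, switching mouse cursor and input mode to match.
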(event Input|EnhancedActionEvents|EnhancedInputActionIA_Move
  (params (ActionValue :type Vector%202D%20Structure) (ElapsedSeconds :type Float%20%28double-precision%29) (TriggeredSeconds :type Float%20%28double-precision%29) (InputAction :type Input%20Action%20Object%20Reference :default "/Game/Input/FP/IA_Move.IA_Move"))
  (bind _returnvalue (Pawn|GetControlledPawn))
  (bind _returnvalue_2 (Transformation|GetActorRotation _returnvalue))
  (Pawn|Input|AddMovementInput _returnvalue (Math|Vector|GetForwardVector (Math|Rotator|MakeRotator 0.0 0.0 (.yaw _returnvalue_2))) (.x ActionValue) false)
  (Pawn|Input|AddMovementInput _returnvalue (Math|Vector|GetRightVector (Math|Rotator|MakeRotator 0.0 0.0 (.yaw _returnvalue_2))) (.y ActionValue) false))

(event Input|EnhancedActionEvents|EnhancedInputActionIA_Look
  (params (ActionValue :type Vector%202D%20Structure) (ElapsedSeconds :type Float%20%28double-precision%29) (TriggeredSeconds :type Float%20%28double-precision%29) (InputAction :type Input%20Action%20Object%20Reference :default "/Game/Input/FP/IA_Look.IA_Look"))
  (bind _returnvalue (Pawn|GetControlledPawn))
  (Pawn|Input|AddControllerYawInput _returnvalue (.x ActionValue))
  (Pawn|Input|AddControllerPitchInput _returnvalue (.y ActionValue)))

(event EventBeginPlay
  (Input|AddMappingContext (PlayerController|LocalPlayerSubsystems|GetEnhancedInputLocalPlayerSubsystem) "/Game/Input/FP/IMC_FP.IMC_FP" 0 "(bIgnoreAllPressedKeysUntilRelease=True,bForceImmediately=False,bNotifyUserSettings=False)"))

(event Input|KeyboardEvents|DebugKeyM
  (params (Key :type Key%20Structure :default "None") (ActionValue :type Input%20Action%20Value%20Structure))
  (bind _returnvalue (Game|GetPlayerController 0))
  (:Pressed
    (Utilities|FlowControl|FlipFlop
      (:A
        (bind _returnvalue_2 (UserInterface|CreateWidget "/Game/UI/WBP_Riddle_1.WBP_Riddle_1_C"))
        (UserInterface|Viewport|AddtoViewport _returnvalue_2 0)
        (Variables|Default|SetbShowMouseCursor true)
        (Input|SetInputModeGameandUI _returnvalue 0 "DoNotLock" true false))
      (:B
        (Widget|RemovefromParent _returnvalue_2)
        (Variables|Default|SetbShowMouseCursor false)
        (Input|SetInputModeGameOnly _returnvalue false)))))

(fn ConstructionScript)