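; Build-mode player character that lets the player place mesh pieces with the mouse cursor once possessed.
; Tick traces from the cursor to position a collision-free preview component using a preview material, storing its transform.
; Input actions cycle the mesh array, rotate the preview, adjust its height offset and spin the camera yaw.
; Placing spawns a BP_Builder at the stored transform with the selected mesh when the cursor trace hits.
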(event Input|EnhancedActionEvents|EnhancedInputActionIA_Place
  (params (ActionValue :type Boolean) (ElapsedSeconds :type Float%20%28double-precision%29) (TriggeredSeconds :type Float%20%28double-precision%29) (InputAction :type Input%20Action%20Object%20Reference :default "/Game/Input/Build/IA_Place.IA_Place"))
  ;[0.15 0.15 0.15 0.5] Place and Build
  (:Started
    (bind _returnvalue (CallFunction|MouseTrace))
    (if _returnvalue
      (bind _returnvalue_2 (Game|SpawnActorfromClass "/Game/Bluprints/Actor/BP_Builder.BP_Builder_C" (Variables|Default|GetBuildTransform) "Undefined" "MultiplyWithRoot" 0 0))
      (Components|StaticMesh|SetStaticMesh (Variables|/Game/Bluprints/Actor/BP_Builder.BP_Builder_C|GetStaticMesh _returnvalue_2) (Utilities|Array|Get(acopy) (Variables|Default|GetBuildMesh) (Variables|Default|GetBuildMeshIndex))))))

(event Input|EnhancedActionEvents|EnhancedInputActionIA_RotateClockWise
  (params (ActionValue :type Boolean) (ElapsedSeconds :type Float%20%28double-precision%29) (TriggeredSeconds :type Float%20%28double-precision%29) (InputAction :type Input%20Action%20Object%20Reference :default "/Game/Input/Build/IA_RotateClockWise.IA_RotateClockWise"))
  ;[0.15 0.15 0.15 0.5] Place and Build
  ;;[0.15 0.15 0.15 0.5] 预览
  ;;;[0.15 0.15 0.15 0.5] 旋转建筑残块
  (Transformation|AddWorldRotation (Variables|Default|GetBuildPreview) (Math|Rotator|MakeRotator 0.0 0.0 5.0) false false))

(event Input|EnhancedActionEvents|EnhancedInputActionIA_RotateCounterClockWise
  (params (ActionValue :type Boolean) (ElapsedSeconds :type Float%20%28double-precision%29) (TriggeredSeconds :type Float%20%28double-precision%29) (InputAction :type Input%20Action%20Object%20Reference :default "/Game/Input/Build/IA_RotateCounterClockWise.IA_RotateCounterClockWise"))
  ;[0.15 0.15 0.15 0.5] Place and Build
  ;;[0.15 0.15 0.15 0.5] 预览
  ;;;[0.15 0.15 0.15 0.5] 旋转建筑残块
  (Transformation|AddWorldRotation (Variables|Default|GetBuildPreview) (Math|Rotator|MakeRotator 0.0 0.0 -5.0) false false))

(event Input|EnhancedActionEvents|EnhancedInputActionIA_CameraSpinA
  (params (ActionValue :type Vector%202D%20Structure) (ElapsedSeconds :type Float%20%28double-precision%29) (TriggeredSeconds :type Float%20%28double-precision%29) (InputAction :type Input%20Action%20Object%20Reference :default "/Game/Input/Build/IA_CameraSpinA.IA_CameraSpinA"))
  (bind _returnvalue (Game|GetPlayerController 0))
  (bind _returnvalue_2 (Game|GetPlayerController 0))
  (bind _returnvalue_3 (Pawn|GetControlRotation _returnvalue :!class /Script/Engine.Controller))
  (bind _returnvalue_4 (Pawn|GetControlRotation _returnvalue_2 :!class /Script/Engine.Controller))
  (bind (_roll _pitch _yaw) (Math|Rotator|BreakRotator _returnvalue_4))
  ;[0.15 0.15 0.15 0.5] 视角
  (Pawn|SetControlRotation _returnvalue (Math|Rotator|MakeRotator (.roll _returnvalue_3) (.pitch _returnvalue_3) (.yaw (Math|Interpolation|RInterpTo _returnvalue_4 (Math|Rotator|MakeRotator _roll _pitch (+ _yaw 1.0)) 0.01 0.0)))))

(event Input|EnhancedActionEvents|EnhancedInputActionIA_BuilderZUP
  (params (ActionValue :type Boolean) (ElapsedSeconds :type Float%20%28double-precision%29) (TriggeredSeconds :type Float%20%28double-precision%29) (InputAction :type Input%20Action%20Object%20Reference :default "/Game/Input/Build/IA_BuilderZUP.IA_BuilderZUP"))
  ;[0.15 0.15 0.15 0.5] Place and Build
  ;;[0.15 0.15 0.15 0.5] 预览
  ;;;[0.15 0.15 0.15 0.5] 改变z轴高度
  (Variables|Default|SetBuilderZPosChange (+ (Variables|Default|GetBuilderZPosChange) 5.0)))

(event Input|EnhancedActionEvents|EnhancedInputActionIA_BuilderZDown
  (params (ActionValue :type Boolean) (ElapsedSeconds :type Float%20%28double-precision%29) (TriggeredSeconds :type Float%20%28double-precision%29) (InputAction :type Input%20Action%20Object%20Reference :default "/Game/Input/Build/IA_BuilderZDown.IA_BuilderZDown"))
  ;[0.15 0.15 0.15 0.5] Place and Build
  ;;[0.15 0.15 0.15 0.5] 预览
  ;;;[0.15 0.15 0.15 0.5] 改变z轴高度
  (Variables|Default|SetBuilderZPosChange (+ (Variables|Default|GetBuilderZPosChange) -5.0)))

(event Input|EnhancedActionEvents|EnhancedInputActionIA_CameraSpinD
  (params (ActionValue :type Vector%202D%20Structure) (ElapsedSeconds :type Float%20%28double-precision%29) (TriggeredSeconds :type Float%20%28double-precision%29) (InputAction :type Input%20Action%20Object%20Reference :default "/Game/Input/Build/IA_CameraSpinD.IA_CameraSpinD"))
  (bind _returnvalue (Game|GetPlayerController 0))
  (bind _returnvalue_2 (Game|GetPlayerController 0))
  (bind _returnvalue_3 (Pawn|GetControlRotation _returnvalue_2 :!class /Script/Engine.Controller))
  (bind _returnvalue_4 (Pawn|GetControlRotation _returnvalue :!class /Script/Engine.Controller))
  (bind (_roll _pitch _yaw) (Math|Rotator|BreakRotator _returnvalue_4))
  ;[0.15 0.15 0.15 0.5] 视角
  (Pawn|SetControlRotation _returnvalue_2 (Math|Rotator|MakeRotator (.roll _returnvalue_3) (.pitch _returnvalue_3) (.yaw (Math|Interpolation|RInterpTo _returnvalue_4 (Math|Rotator|MakeRotator _roll _pitch (- _yaw 1.0)) 0.01 0.0)))))

(event Input|EnhancedActionEvents|EnhancedInputActionIA_SelectBuilderMesh
  (params (ActionValue :type Float%20%28double-precision%29) (ElapsedSeconds :type Float%20%28double-precision%29) (TriggeredSeconds :type Float%20%28double-precision%29) (InputAction :type Input%20Action%20Object%20Reference :default "/Game/Input/Build/IA_SelectBuilderMesh.IA_SelectBuilderMesh"))
  (bind _buildmesh (Variables|Default|GetBuildMesh))
  (bind _buildpreview (Variables|Default|GetBuildPreview))
  (bind _returnvalue (Utilities|Array|Length _buildmesh))
  ;[0.15 0.15 0.15 0.5] Place and Build
  ;;[0.15 0.15 0.15 0.5] 预览
  ;;;[0.15 0.15 0.15 0.5] 选择建筑残块
  (if (> ActionValue 0.0)
    (Variables|Default|SetLastMeshIndex (Variables|Default|GetBuildMeshIndex))
    (Math|Integer|IncrementInt (Variables|Default|GetBuildMeshIndex)
      (:%20%20
        (Variables|Default|SetBuildMeshIndex (Math|Integer|%(Integer) (Variables|Default|GetBuildMeshIndex) _returnvalue))
        (CallFunction|ChangePreviewBuild _buildpreview)))
    (else
      (bind _output_get (Variables|Default|SetLastMeshIndex (Variables|Default|GetBuildMeshIndex)))
      (if (== _output_get 0)
        (Variables|Default|SetBuildMeshIndex (- _returnvalue 1))
        (CallFunction|ChangePreviewBuild _buildpreview)
        (else
          (Math|Integer|DecrementInt (Variables|Default|GetBuildMeshIndex)
            (:%20%20
              (CallFunction|ChangePreviewBuild _buildpreview))))))))

(event EventPossessed
  (params (NewController :type Controller%20Object%20Reference))
  (bind _returnvalue (Game|GetPlayerController 0))
  ;[0.15 0.15 0.15 0.5] Init
  (Utilities|IsValid _returnvalue :!label _label
    (:Is%20Valid
      (Variables|/Script/Engine.PlayerController|SetbShowMouseCursor _returnvalue true)
      (Variables|Default|SetControlled? true)
      (Variables|Default|SetBuildPreview 0))
    (:Is%20Not%20Valid
      (Utilities|FlowControl|DelayUntilNextTick)
      (goto _label))))

(event EventTick
  (params (DeltaSeconds :type Float%20%28single-precision%29))
  ;[0.15 0.15 0.15 0.5] Place and Build
  ;;[0.15 0.15 0.15 0.5] 预览
  (if (Variables|Default|GetControlled?)
    (bind (_returnvalue _outhit) (CallFunction|MouseTrace))
    (if _returnvalue
      (if (Utilities|IsValid (Variables|Default|GetBuildPreview))
        (Transformation|SetWorldLocation (Variables|Default|GetBuildPreview) (Math|Vector|MakeVector (.X (Math|Vector|BreakVector (.Location (Collision|BreakHitResult _outhit)))) (.Y (Math|Vector|BreakVector (.Location (Collision|BreakHitResult _outhit)))) (+ (.Z (Math|Vector|BreakVector (.Location (Collision|BreakHitResult _outhit)))) (Variables|Default|GetBuilderZPosChange))) false false)
        (Variables|Default|SetBuildTransform (Transformation|GetWorldTransform (Variables|Default|GetBuildPreview)))
        (else
          (bind _returnvalue_2 (Game|AddComponentbyClass "/Script/Engine.StaticMeshComponent" false))
          (bind _output_get (Variables|Default|SetBuildPreview _returnvalue_2))
          (Collision|SetCollisionEnabled _output_get "NoCollision")
          (CallFunction|ChangePreviewBuild _output_get))))))

(fn ConstructionScript
  (|CallParentFunction))

(fn MouseTrace
  (bind _returnvalue (Game|GetPlayerController 0))
  (bind (_worldlocation _worlddirection) (Game|Player|ConvertMouseLocationToWorldSpace _returnvalue))
  (bind (_outhit _returnvalue_2) (Collision|LineTraceByChannel _worldlocation (+ _worldlocation (* _worlddirection 1e+04)) "TraceTypeQuery1" false 0 "None"))
  (return _returnvalue_2 _outhit))

(fn ChangePreviewBuild
  (params (PreviewBuild :type Static%20Mesh%20Component%20Object%20Reference))
  (bind _buildpreview (Variables|Default|GetBuildPreview))
  (Components|StaticMesh|SetStaticMesh PreviewBuild (Utilities|Array|Get(acopy) (Variables|Default|GetBuildMesh) (Variables|Default|GetBuildMeshIndex)))
  (for (_ _array_index) (Rendering|Material|GetMaterials _buildpreview)
    (Rendering|Material|SetMaterial _buildpreview _array_index "/Game/Materials/M_BuildPreview.M_BuildPreview")))

(fn SetBuildMeshes
  (params (0 :type Static%20Mesh%20Object%20Reference) (1 :type Static%20Mesh%20Object%20Reference) (2 :type Static%20Mesh%20Object%20Reference) (3 :type Static%20Mesh%20Object%20Reference) (4 :type Static%20Mesh%20Object%20Reference) (5 :type Static%20Mesh%20Object%20Reference))
  (bind _buildmesh (Variables|Default|GetBuildMesh))
  (bind _buildmesh_2 (Variables|Default|GetBuildMesh))
  (Utilities|Array|SetArrayElem _buildmesh 0 0)
  (Utilities|Array|SetArrayElem _buildmesh 0 1)
  (Utilities|Array|SetArrayElem _buildmesh 0 2)
  (Utilities|Array|SetArrayElem _buildmesh_2 0 3)
  (Utilities|Array|SetArrayElem _buildmesh_2 0 4)
  (Utilities|Array|SetArrayElem _buildmesh_2 0 5))