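; First-person player character Blueprint that handles Enhanced Input move and look, forwards interact presses to the current interact actor, and shows a visit widget on BeginPlay.
; Q triggers the level 1-to-3 transition, flip-flopping a camera blend between PaintCam and the player while replacing the visit widget with 3UI and enabling the cursor.
; Key 9 triggers a sunset by showing volumetric clouds, hiding the skybox and retuning the directional light.
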(event Input|EnhancedActionEvents|EnhancedInputActionIA_Interact
  (params (ActionValue :type Boolean) (ElapsedSeconds :type Float%20%28double-precision%29) (TriggeredSeconds :type Float%20%28double-precision%29) (InputAction :type Input%20Action%20Object%20Reference :default "/Game/Input/FP/IA_Interact.IA_Interact"))
  (:Started
    (Class|BPIInteract|Interact(Message) (Variables|Default|GetCurInteractActor))))

(event Input|EnhancedActionEvents|EnhancedInputActionIA_Move
  (params (ActionValue :type Vector%202D%20Structure) (ElapsedSeconds :type Float%20%28double-precision%29) (TriggeredSeconds :type Float%20%28double-precision%29) (InputAction :type Input%20Action%20Object%20Reference :default "/Game/Input/FP/IA_Move.IA_Move"))
  (bind _self self)
  (bind _returnvalue (Transformation|GetActorRotation _self))
  (Pawn|Input|AddMovementInput _self (Math|Vector|GetForwardVector (Math|Rotator|MakeRotator 0.0 0.0 (.yaw _returnvalue))) (.x ActionValue) false)
  (Pawn|Input|AddMovementInput _self (Math|Vector|GetRightVector (Math|Rotator|MakeRotator 0.0 0.0 (.yaw _returnvalue))) (.y ActionValue) false))

(event Input|EnhancedActionEvents|EnhancedInputActionIA_Look
  (params (ActionValue :type Vector%202D%20Structure) (ElapsedSeconds :type Float%20%28double-precision%29) (TriggeredSeconds :type Float%20%28double-precision%29) (InputAction :type Input%20Action%20Object%20Reference :default "/Game/Input/FP/IA_Look.IA_Look"))
  (bind _self self)
  (Pawn|Input|AddControllerYawInput _self (.x ActionValue))
  (Pawn|Input|AddControllerPitchInput _self (.y ActionValue)))

(event EventBeginPlay
  (|CallParentFunction)
  (Utilities|FlowControl|Sequence
    (:then_0
      (bind _asbp_controller (Utilities|Casting|CastToBP_Controller (Pawn|GetController)))
      (Variables|Default|SetAs%20BP%20Controller _asbp_controller))
    (:then_1
      (bind _returnvalue (UserInterface|CreateWidget "/Game/UI/WBP_Visit.WBP_Visit_C"))
      (bind _output_get (Variables|Default|Set1%20UI%20Inst _returnvalue))
      (UserInterface|Viewport|AddtoViewport _output_get 0))))

(event Collision|EventActorBeginOverlap
  (params (OtherActor :type Actor%20Object%20Reference))
  (|CallParentFunction OtherActor) ; 此节点被禁用，将不会被调用。\n从引脚连出引线来编译功能。
)

(event EventTick
  (params (DeltaSeconds :type Float%20%28single-precision%29))
  (|CallParentFunction DeltaSeconds) ; 此节点被禁用，将不会被调用。\n从引脚连出引线来编译功能。
)

(event EventPossessed
  (params (NewController :type Controller%20Object%20Reference)))

(event Custom|Sunset
  (Utilities|FlowControl|Sequence
    (:then_0
      (bind _returnvalue (Actor|GetActorOfClass "/Script/Engine.VolumetricCloud"))
      (Rendering|SetVisibility (Variables|/Script/Engine.VolumetricCloud|GetVolumetricCloudComponent _returnvalue) true false)
      (Rendering|SetActorHiddenInGame _returnvalue false)
      (bind _returnvalue_2 (Actor|GetActorOfClass "/Game/sky/skybox.skybox_C"))
      (Rendering|SetActorHiddenInGame _returnvalue_2 true))
    (:then_1
      (bind _returnvalue_3 (Actor|GetActorOfClass "/Script/Engine.DirectionalLight"))
      (Utilities|IsValid (Actor|GetComponentbyClass _returnvalue_3 "/Script/Engine.DirectionalLightComponent")
        (:Is%20Valid
          (Development|PrintString "Hello")
          (Class|DirectionalLightComponent|SetLightSourceAngle (Actor|GetComponentbyClass _returnvalue_3 "/Script/Engine.DirectionalLightComponent") 15.0)
          (Rendering|Components|Light|SetLightColor (Actor|GetComponentbyClass _returnvalue_3 "/Script/Engine.DirectionalLightComponent") "(R=1.000000,G=0.404762,B=0.062500,A=1.000000)" true)
          (Transformation|SetWorldRotation (Actor|GetComponentbyClass _returnvalue_3 "/Script/Engine.DirectionalLightComponent") "-8.000000,0.000000,0.000000" false false)
          (Rendering|Components|Light|SetIntensity (Actor|GetComponentbyClass _returnvalue_3 "/Script/Engine.DirectionalLightComponent") 5.0))))))

(event Custom|1%20To%203
  (bind _returnvalue (Game|GetPlayerController 0))
  (bind _returnvalue_2 (Game|GetPlayerController 0))
  ;[0.15 0.15 0.15 0.5] 第一关至第三关
  (Utilities|FlowControl|Sequence
    (:then_0
      (Utilities|FlowControl|FlipFlop
        (:A
          (Game|Player|SetViewTargetwithBlend _returnvalue (Variables|Default|GetPaintCam) 2.0 "VTBlend_Cubic" 0.0 false))
        (:B
          (Game|Player|SetViewTargetwithBlend _returnvalue self 1.0 "VTBlend_Cubic" 0.0 false))))
    (:then_1
      (bind _returnvalue_3 (UserInterface|CreateWidget (Variables|Default|Get3%20UI)))
      (UserInterface|Viewport|AddtoViewport _returnvalue_3 0)
      (Variables|/Script/Engine.PlayerController|SetbShowMouseCursor _returnvalue_2 true)
      (Input|SetInputModeGameandUI _returnvalue_2 0 "DoNotLock" true false)
      (bind _1_ui_inst (Variables|Default|Get1%20UI%20Inst)
        (:then
          (Widget|RemovefromParent _1_ui_inst))
        (:else)))))

(event Input|KeyboardEvents|Q
  (params (Key :type Key%20Structure :default "None"))
  (:Pressed
    (CallFunction|1to3)))

(event Input|KeyboardEvents|9
  (params (Key :type Key%20Structure :default "None"))
  ;[0.15 0.15 0.15 0.5] 夕阳
  (:Pressed
    (CallFunction|Sunset)))

(fn ConstructionScript
  (|CallParentFunction))

(fn ChangeCurInteractActor
  (params (InteractActor :type Actor%20Object%20Reference))
  (Utilities|IsValid InteractActor
    (:Is%20Valid
      (Variables|Default|SetCurInteractActor InteractActor))
    (:Is%20Not%20Valid
      (Variables|Default|SetCurInteractActor 0))))