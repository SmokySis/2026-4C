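; Player pawn for the sunmao (mortise-and-tenon) assembly puzzle in three levels: YanWeiSun, WoodBridge and DouGong.
; On possession it swaps input mapping, spawns joint pieces from linked DataTable rows at component transforms, and adds level UI and depth of field.
; Axis input slides the selected unfinished piece along a level- or piece-specific axis.
; When all pieces finish, it shows an end widget, then reveals build chunks and hands control to BP_Character_Build.
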(event Custom|SunMaoOver
  (bind _startlocation (Variables|Default|GetStartLocation))
  ;[0.15 0.15 0.15 0.5] 拼接结束
  (Widget|RemovefromParent (Variables|Default|GetSunMaoUI%20))
  (Widget|RemovefromParent (Variables|Default|GetSecondaryView))
  (Variables|Default|SetCurJoint 0)
  (Utilities|FlowControl|Sequence
    (:then_0
      (Utilities|FlowControl|Delay 6.0)
      (Audio|PlaySound2D "/Game/_Asset/SFX/Book_page_flip_1.Book_page_flip_1" 1.0 1.0 0.0 0 0)
      (bind _outactors (Actor|GetAllActorsOfClass "/Game/_BP/BuildChunks/BP_BuildChunk_Base.BP_BuildChunk_Base_C"))
      (for _array_element _outactors
        (Rendering|SetActorHiddenInGame _array_element false)
        (bind _returnvalue (Game|SpawnActorfromClass "/Game/Bluprints/Characters/Player/BP_Character_Build.BP_Character_Build_C" (Math|Transform|MakeTransform (Utilities|Select :Index (Variables|/Game/Bluprints/Game/GI_GameInstance.GI_GameInstance_C|GetLevelIndex (.AsGI%20Game%20Instance (Utilities|Casting|CastToGI_GameInstance (Game|GetGameInstance)))) :NewEnumerator0 (Utilities|Array|Get(acopy) _startlocation) :NewEnumerator1 (Utilities|Array|Get(acopy) _startlocation 1) :NewEnumerator2 (Utilities|Array|Get(acopy) _startlocation 2)) "0.000000,90.000000,0.000000" "1.000000,1.000000,1.000000") "Undefined" "MultiplyWithRoot" 0 0))
        (Widget|RemovefromParent (Variables|Default|GetOver%20UI))
        (Pawn|Possess (Game|GetPlayerController 0) _returnvalue)
        (Actor|DestroyActor)))
    (:then_1
      (bind _asgi_game_instance (Utilities|Casting|CastToGI_GameInstance (Game|GetGameInstance)))
      (Audio|PlaySound2D "/Game/_Asset/SFX/Book_page_flip_1.Book_page_flip_1" 1.0 1.0 0.0 0 0)
      (switch Utilities|FlowControl|Switch|SwitchonEnum_LevelIndex (Variables|/Game/Bluprints/Game/GI_GameInstance.GI_GameInstance_C|GetLevelIndex _asgi_game_instance)
        (:NewEnumerator0
          (CallFunction|CreateOverUI "/Game/UI/WBP_SM_Over_1.WBP_SM_Over_1_C"))
        (:NewEnumerator1
          (CallFunction|CreateOverUI "/Game/UI/WBP_SM_Over_2.WBP_SM_Over_2_C"))
        (:NewEnumerator2
          (CallFunction|CreateOverUI "/Game/UI/WBP_SM_Over_3.WBP_SM_Over_3_C"))))))

(event Custom|SunMaoBegin
  (bind _returnvalue (Game|GetPlayerController 0))
  (bind _returnvalue_2 (PlayerController|LocalPlayerSubsystems|GetEnhancedInputLocalPlayerSubsystem _returnvalue))
  ;[0.15 0.15 0.15 0.5] 创建并初始化榫卯
  (Input|RemoveMappingContext _returnvalue_2 "/Game/Input/FP/IMC_FP.IMC_FP" "(bIgnoreAllPressedKeysUntilRelease=True,bForceImmediately=False,bNotifyUserSettings=False)")
  (Input|AddMappingContext _returnvalue_2 "/Game/Input/Joint/IM_JointControll.IM_JointControll" 0 "(bIgnoreAllPressedKeysUntilRelease=True,bForceImmediately=False,bNotifyUserSettings=False)")
  (Variables|/Script/Engine.PlayerController|SetbShowMouseCursor (Game|GetPlayerController 0) true)
  (bind _asgi_game_instance (Utilities|Casting|CastToGI_GameInstance (Game|GetGameInstance)))
  (switch Utilities|FlowControl|Switch|SwitchonEnum_LevelIndex (Variables|/Game/Bluprints/Game/GI_GameInstance.GI_GameInstance_C|GetLevelIndex _asgi_game_instance)
    (:NewEnumerator0
      (|YanWeiSunInit))
    (:NewEnumerator1
      (|WoodBridge))
    (:NewEnumerator2
      (|DouGongInit))))

(event Input|EnhancedActionEvents|EnhancedInputActionIA_SunMaoMoveX
  (params (ActionValue :type Float%20%28double-precision%29) (ElapsedSeconds :type Float%20%28double-precision%29) (TriggeredSeconds :type Float%20%28double-precision%29) (InputAction :type Input%20Action%20Object%20Reference :default "/Game/Input/Joint/IA_SunMaoMoveX.IA_SunMaoMoveX"))
  (bind _curjoint (Variables|Default|GetCurJoint))
  ;[0.15 0.15 0.15 0.5] 榫卯移动
  (Utilities|IsValid _curjoint
    (:Is%20Valid
      (if (not (Variables|/Game/_BP/SunMao/BP_SunMao_Base.BP_SunMao_Base_C|GetIsOver? (.AsBP%20Sun%20Mao%20Base (Utilities|Casting|CastToBP_SunMao_Base _curjoint))))
        (switch Utilities|FlowControl|Switch|SwitchonEnum_LevelIndex (Variables|/Game/Bluprints/Game/GI_GameInstance.GI_GameInstance_C|GetLevelIndex (.AsGI%20Game%20Instance (Utilities|Casting|CastToGI_GameInstance (Game|GetGameInstance))))
          (:NewEnumerator0
            (|YanWeiSunMove ActionValue))
          (:NewEnumerator1
            (|WoodBridgeMove ActionValue ActionValue ActionValue))
          (:NewEnumerator2
            (|DouGongMove ActionValue)))))))

(event Collision|EventActorBeginOverlap
  (params (OtherActor :type Actor%20Object%20Reference)))

(event EventTick
  (params (DeltaSeconds :type Float%20%28single-precision%29)))

(event EventPossessed
  (params (NewController :type Controller%20Object%20Reference))
  ;[0.15 0.15 0.15 0.5] 创建并初始化榫卯
  (Utilities|FlowControl|Delay 0.2)
  (CallFunction|SunMaoBegin))

(fn ConstructionScript)

(fn PreCreateandInitJoints
  (params (SunMaoInfoInfoRow :type Name))
  (bind _returnvalue (Utilities|GetDataTableRow "/Game/_BP/SunMao/DT_SunMaoInfoInfo.DT_SunMaoInfoInfo" SunMaoInfoInfoRow)
    (:then
      (CallFunction|CreateandInitJoints (.StartRow (Utilities|Struct|BreakS_SunMaoInfoInfo _returnvalue)) (.EndRow (Utilities|Struct|BreakS_SunMaoInfoInfo _returnvalue))))))

(fn SetJointsLocationbySelf
  (params (Forward :type Float%20%28double-precision%29) (Right :type Float%20%28double-precision%29))
  (bind _self self)
  (bind _returnvalue (Transformation|GetActorRotation _self))
  (return (+ (* (Math|Vector|GetRightVector _returnvalue) Right) (+ (* (Math|Vector|GetForwardVector _returnvalue) Forward) (Transformation|GetActorLocation _self)))))

(fn CreateandInitJoints
  (params (StartRow :type Name) (EndRow :type Name))
  (bind _asgi_game_instance (Utilities|Casting|CastToGI_GameInstance (Game|GetGameInstance)))
  (switch Utilities|FlowControl|Switch|SwitchonEnum_LevelIndex (Variables|/Game/Bluprints/Game/GI_GameInstance.GI_GameInstance_C|GetLevelIndex _asgi_game_instance)
    (:NewEnumerator0
      (|GetSunMaoTransforms1))
    (:NewEnumerator1
      (|GetWoodBridgeTransform))
    (:NewEnumerator2
      (|GetSunMaoTransform)))
  (LocalVariables|SetStartRowName StartRow)
  (LocalVariables|SetEndRowName EndRow)
  (LocalVariables|SetCurRow (LocalVariables|GetStartRowName))
  (while (not (== (LocalVariables|GetLastRow) (LocalVariables|GetEndRowName)))
    (bind _returnvalue (Utilities|GetDataTableRow "/Game/_BP/SunMao/DT_SunMaoInfo.DT_SunMaoInfo" (LocalVariables|GetCurRow))
      (:then
        (LocalVariables|SetLastRow (LocalVariables|GetCurRow))
        (LocalVariables|SetCurRow (.NextRowName (Utilities|Struct|BreakS_SunMaoInfo _returnvalue)))
        (bind _returnvalue_2 (Game|SpawnActorfromClass (.SunMaoClass (Utilities|Struct|BreakS_SunMaoInfo _returnvalue)) (Utilities|Array|Get(acopy) (LocalVariables|GetSunMaoTransforms) (LocalVariables|GetSunMaoIndex)) "AlwaysSpawn" "MultiplyWithRoot" 0 0))
        (Math|Integer|IncrementInt (LocalVariables|GetSunMaoIndex)
          (:%20%20
            (Utilities|Array|Add (Variables|Default|GetJointArr) _returnvalue_2)))))))

(fn SetControlledSunMao
  (params (SunMaoIndex :type Integer))
  (bind _output_get (Variables|Default|SetCurJoint (Utilities|Array|Get(acopy) (Variables|Default|GetJointArr) SunMaoIndex)))
  (Development|PrintString (Utilities|GetDisplayName _output_get)))

(fn SetDepthOfFeild
  (bind _returnvalue (AddComponent|AddPostProcessComponent false))
  (Utilities|Struct|SetmembersinPostProcessSettings (Variables|/Script/Engine.PostProcessComponent|GetSettings _returnvalue) 0.2 24.576 (Math|Vector|VectorLength (- (Transformation|GetWorldLocation (Variables|Default|GetCamera)) (Transformation|GetWorldLocation (Variables|Default|GetWoodBridge0))))))

(fn CheckIsOver?
  (for _array_element (Variables|Default|GetJointArr)
    (if (not (Variables|/Game/_BP/SunMao/BP_SunMao_Base.BP_SunMao_Base_C|GetIsOver? (.AsBP%20Sun%20Mao%20Base (Utilities|Casting|CastToBP_SunMao_Base _array_element))))
      (LocalVariables|SetTotalOver? false)))
  (if (LocalVariables|GetTotalOver?)
    (CallFunction|SunMaoOver)))

(fn CreateOverUI
  (params (UIClass :type User%20Widget%20Class%20Reference))
  (bind _returnvalue (UserInterface|CreateWidget UIClass (Game|GetPlayerController 0)))
  (bind _output_get (Variables|Default|SetOver%20UI _returnvalue))
  (UserInterface|Viewport|AddtoViewport _output_get 0))