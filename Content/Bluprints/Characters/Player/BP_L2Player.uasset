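; Player Blueprint for mouse-driven placement of a couch mesh, with a rotatable spring arm camera.
; Each Tick, a Visibility trace from the cursor moves a lazily created preview mesh, tinted with a preview material, and caches its transform.
; Enhanced Input rotates the preview or spring arm, and the build action spawns a movable StaticMeshActor at the cached transform when the trace hits.
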(event Input|EnhancedActionEvents|EnhancedInputActionIA_Build
  (params (ActionValue :type Boolean) (ElapsedSeconds :type Float%20%28double-precision%29) (TriggeredSeconds :type Float%20%28double-precision%29) (InputAction :type Input%20Action%20Object%20Reference :default "/Game/Input/IA_Build.IA_Build"))
  (:Started
    (bind _returnvalue (CallFunction|MouseTrace))
    (if _returnvalue
      (bind _returnvalue_2 (Game|SpawnActorfromClass "/Script/Engine.StaticMeshActor" (Variables|Default|GetBuildTransform) "Undefined" "MultiplyWithRoot" 0 0))
      (Transformation|SetMobility _returnvalue_2 "Movable")
      (Components|StaticMesh|SetStaticMesh (Variables|/Script/Engine.StaticMeshActor|GetStaticMeshComponent _returnvalue_2) "/Game/StarterContent/Props/SM_Couch.SM_Couch"))))

(event Input|EnhancedActionEvents|EnhancedInputActionIA_RotateClockWise
  (params (ActionValue :type Boolean) (ElapsedSeconds :type Float%20%28double-precision%29) (TriggeredSeconds :type Float%20%28double-precision%29) (InputAction :type Input%20Action%20Object%20Reference :default "/Game/Input/IA_RotateClockWise.IA_RotateClockWise"))
  (Transformation|AddWorldRotation (Variables|Default|GetBuildPreview) (Math|Rotator|MakeRotator 0.0 0.0 5.0) false false))

(event Input|EnhancedActionEvents|EnhancedInputActionIA_RotateCounterClockWise
  (params (ActionValue :type Boolean) (ElapsedSeconds :type Float%20%28double-precision%29) (TriggeredSeconds :type Float%20%28double-precision%29) (InputAction :type Input%20Action%20Object%20Reference :default "/Game/Input/IA_RotateCounterClockWise.IA_RotateCounterClockWise"))
  (Transformation|AddWorldRotation (Variables|Default|GetBuildPreview) (Math|Rotator|MakeRotator 0.0 0.0 -5.0) false false))

(event Input|EnhancedActionEvents|EnhancedInputActionIA_SpringArmRotate
  (params (ActionValue :type Float%20%28double-precision%29) (ElapsedSeconds :type Float%20%28double-precision%29) (TriggeredSeconds :type Float%20%28double-precision%29) (InputAction :type Input%20Action%20Object%20Reference :default "/Game/Input/IA_SpringArmRotate.IA_SpringArmRotate"))
  (Development|PrintString (Utilities|String|ToString(Float) ActionValue))
  (Transformation|AddWorldRotation (Variables|Default|GetSpringArm) (Math|Rotator|MakeRotator 0.0 0.0 (* ActionValue 2.0)) false false))

(event EventBeginPlay
  (bind _returnvalue (Game|GetPlayerController 0))
  (Variables|/Script/Engine.PlayerController|SetbShowMouseCursor _returnvalue true)
  (Input|AddMappingContext (PlayerController|LocalPlayerSubsystems|GetEnhancedInputLocalPlayerSubsystem _returnvalue) "/Game/Input/IM_Building.IM_Building" 0 "(bIgnoreAllPressedKeysUntilRelease=True,bForceImmediately=False,bNotifyUserSettings=False)"))

(event Collision|EventActorBeginOverlap
  (params (OtherActor :type Actor%20Object%20Reference)))

(event EventTick
  (params (DeltaSeconds :type Float%20%28single-precision%29))
  (bind (_returnvalue _outhit) (CallFunction|MouseTrace))
  (if _returnvalue
    (if (Utilities|IsValid (Variables|Default|GetBuildPreview))
      (Transformation|SetWorldLocation (Variables|Default|GetBuildPreview) (.Location (Collision|BreakHitResult _outhit)) false false)
      (Variables|Default|SetBuildTransform (Transformation|GetWorldTransform (Variables|Default|GetBuildPreview)))
      (else
        (bind _returnvalue_2 (Game|AddComponentbyClass "/Script/Engine.StaticMeshComponent" false))
        (bind _output_get (Variables|Default|SetBuildPreview _returnvalue_2))
        (Components|StaticMesh|SetStaticMesh _output_get "/Game/StarterContent/Props/SM_Couch.SM_Couch")
        (for (_ _array_index) (Rendering|Material|GetMaterials (Variables|Default|GetBuildPreview))
          (Rendering|Material|SetMaterial (Variables|Default|GetBuildPreview) _array_index "/Game/Materials/M_BuildPreview.M_BuildPreview"))))))

(fn ConstructionScript)

(fn MouseTrace
  (bind _returnvalue (Game|GetPlayerController 0))
  (bind (_worldlocation _worlddirection) (Game|Player|ConvertMouseLocationToWorldSpace _returnvalue))
  (bind (_outhit _returnvalue_2) (Collision|LineTraceByChannel _worldlocation (+ (* _worlddirection 1e+04) _worldlocation) "TraceTypeQuery1" false 0 "None"))
  (return _returnvalue_2 _outhit))