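; BP_GM_Build is the build-mode GM Blueprint (likely a game mode), setting up player input for building.
; GMInit casts player controller 0 to BP_Controller, caches it and sets the sub-level state.
; It then adds the general and build Enhanced Input mapping contexts at equal priority.
; BeginPlay, Tick and the construction script add no logic of their own.
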(event EventBeginPlay
  (|CallParentFunction) ; 此节点被禁用，将不会被调用。\n从引脚连出引线来编译功能。
)

(event EventTick
  (params (DeltaSeconds :type Float%20%28single-precision%29))
  (|CallParentFunction DeltaSeconds) ; 此节点被禁用，将不会被调用。\n从引脚连出引线来编译功能。
)

(fn ConstructionScript
  (|CallParentFunction))

(fn GMInit
  (bind _asbp_controller (Utilities|Casting|CastToBP_Controller (Game|GetPlayerController 0)))
  (Variables|Default|SetAs%20BP%20Controller _asbp_controller)
  (Variables|Default|SetSubLevelState "NewEnumerator1")
  (Input|AddMappingContext (PlayerController|LocalPlayerSubsystems|GetEnhancedInputLocalPlayerSubsystem (Variables|Default|GetAs%20BP%20Controller)) "/Game/Input/General/IM_General.IM_General" 0 "(bIgnoreAllPressedKeysUntilRelease=True,bForceImmediately=False,bNotifyUserSettings=False)")
  (Input|AddMappingContext (PlayerController|LocalPlayerSubsystems|GetEnhancedInputLocalPlayerSubsystem (Variables|Default|GetAs%20BP%20Controller)) "/Game/Input/Build/IMC_Build.IMC_Build" 0 "(bIgnoreAllPressedKeysUntilRelease=True,bForceImmediately=False,bNotifyUserSettings=False)"))