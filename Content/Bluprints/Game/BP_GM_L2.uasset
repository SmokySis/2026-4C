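; BP_GM_L2 is the level 2 game mode that sequences its gameplay phases: first-person, building, joint play and riddle.
; Each phase event blends the camera to that phase's actor, waits, then has the player controller switch possession and input mappings and updates SubLevelState.
; The Build phase also sets spring arm length and JiangNan building meshes, while JointPlay initializes a joint pair.
; A separate event opens level 3.
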(event Custom|JointPlayBegin
  (bind _as_bp_controller (Variables|Default|GetAs%20BP%20Controller))
  ;[0.15 0.15 0.15 0.5] 从Build过度到JointPlay,并切换控制以及重设输入映射
  (bind _returnvalue (Actor|GetActorOfClass "/Game/Bluprints/Characters/Player/BP_JointControll.BP_JointControll_C"))
  (Game|Player|SetViewTargetwithBlend _as_bp_controller _returnvalue 2.5 "VTBlend_Cubic" 0.0 false)
  (Utilities|FlowControl|Delay 3.0)
  (Default|SwitchPossess _as_bp_controller (Pawn|GetControlledPawn _as_bp_controller) _returnvalue "/Game/Input/Build/IMC_Build.IMC_Build" "/Game/Input/Joint/IM_JointControll.IM_JointControll")
  (Default|CreateandInitJointArr _returnvalue "/Game/ASIAN_Village/StaticMeshes/SM_Acc2Group_bag1.SM_Acc2Group_bag1" "/Game/ASIAN_Village/StaticMeshes/SM_Acc2Group_bag3.SM_Acc2Group_bag3")
  (Variables|Default|SetSubLevelState "NewEnumerator3"))

(event Custom|RiddleBegin
  (bind _as_bp_controller (Variables|Default|GetAs%20BP%20Controller))
  ;[0.15 0.15 0.15 0.5] 从Joint Play过渡到Riddle，并切换输入及重设输入映射
  (bind _returnvalue (Actor|GetActorOfClass "/Game/Bluprints/Characters/Player/BP_Character_Riddle.BP_Character_Riddle_C"))
  (Game|Player|SetViewTargetwithBlend _as_bp_controller _returnvalue 2.5 "VTBlend_Linear" 0.0 false)
  (Utilities|FlowControl|Delay 3.0)
  (Default|SwitchPossess _as_bp_controller (Pawn|GetControlledPawn _as_bp_controller) _returnvalue "/Game/Input/Joint/IM_JointControll.IM_JointControll")
  (Variables|Default|SetSubLevelState "NewEnumerator2"))

(event Custom|BuildBegin
  (bind _as_bp_controller (Variables|Default|GetAs%20BP%20Controller))
  ;[0.15 0.15 0.15 0.5] 从FP过渡到Build，并切换控制以及重设输入映射
  (bind _returnvalue (Actor|GetActorOfClass "/Game/Bluprints/Characters/Player/BP_Character_Build.BP_Character_Build_C"))
  (Game|Player|SetViewTargetwithBlend _as_bp_controller _returnvalue 2.5 "VTBlend_Cubic" 0.0 false)
  (Utilities|FlowControl|Delay 3.0)
  (Default|SwitchPossess _as_bp_controller (Pawn|GetControlledPawn _as_bp_controller) _returnvalue "/Game/Input/FP/IMC_FP.IMC_FP" "/Game/Input/Build/IMC_Build.IMC_Build")
  (Default|SetSpringArmLen _returnvalue 3.5e+03)
  (Default|SetBuildMeshes _returnvalue "/Game/MeshAssets/BuildChunks/JiangNan/SM_Build_JiangNan_1_8A832F30.SM_Build_JiangNan_1_8A832F30" "/Game/MeshAssets/BuildChunks/JiangNan/SM_Build_JiangNan_5.SM_Build_JiangNan_5" "/Game/MeshAssets/BuildChunks/JiangNan/SM_Build_JiangNan_4.SM_Build_JiangNan_4" "/Game/MeshAssets/BuildChunks/JiangNan/SM_Build_JiangNan_2_2CD96C03.SM_Build_JiangNan_2_2CD96C03" "/Game/MeshAssets/BuildChunks/JiangNan/SM_Build_JiangNan_3_AF5DD1A8.SM_Build_JiangNan_3_AF5DD1A8" "/Game/MeshAssets/BuildChunks/JiangNan/SM_JiangNan_Build_0_9F22D4E7.SM_JiangNan_Build_0_9F22D4E7")
  (Variables|Default|SetSubLevelState "NewEnumerator1"))

(event Custom|LoadLevel3
  (Game|OpenLevel(byName) "level_3"))

(event EventBeginPlay
  (|CallParentFunction))

(event EventTick
  (params (DeltaSeconds :type Float%20%28single-precision%29)))

(fn ConstructionScript)