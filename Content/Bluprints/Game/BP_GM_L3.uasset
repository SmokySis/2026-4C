(event Custom|JointPlayBegin
  (bind _as_bp_controller (Variables|Default|GetAs%20BP%20Controller))
  ;[0.15 0.15 0.15 0.5] 从Build过度到JointPlay,并切换控制以及重设输入映射
  (bind _returnvalue (Actor|GetActorOfClass "/Game/Bluprints/Characters/Player/BP_JointControll.BP_JointControll_C"))
  (Game|Player|SetViewTargetwithBlend _as_bp_controller _returnvalue 2.5 "VTBlend_Cubic" 0.0 false)
  (Utilities|FlowControl|Delay 3.0)
  (Default|SwitchPossess _as_bp_controller (Pawn|GetControlledPawn _as_bp_controller) _returnvalue "/Game/Input/Build/IMC_Build.IMC_Build" "/Game/Input/Joint/IM_JointControll.IM_JointControll")
  (Default|CreateandInitJointArr _returnvalue "/Game/ASIAN_Village/StaticMeshes/SM_Acc2Group_bag1.SM_Acc2Group_bag1" "/Game/ASIAN_Village/StaticMeshes/SM_Acc2Group_bag3.SM_Acc2Group_bag3")
  (Variables|Default|SetSubLevelState "NewEnumerator3"))

(event Custom|RiddleBegin
  (bind _as_bp_controller (Variables|Default|GetAs%20BP%20Controller))
  ;[0.15 0.15 0.15 0.5] 从Joint Play过渡到Riddle，并切换输入及重设输入映射
  (bind _returnvalue (Actor|GetActorOfClass "/Game/Bluprints/Characters/Player/BP_Character_Riddle.BP_Character_Riddle_C"))
  (Game|Player|SetViewTargetwithBlend _as_bp_controller _returnvalue 2.5 "VTBlend_Linear" 0.0 false)
  (Utilities|FlowControl|Delay 3.0)
  (Default|SwitchPossess _as_bp_controller (Pawn|GetControlledPawn _as_bp_controller) _returnvalue "/Game/Input/Joint/IM_JointControll.IM_JointControll")
  (Variables|Default|SetSubLevelState "NewEnumerator2"))

(event Custom|BuildBegin
  (bind _as_bp_controller (Variables|Default|GetAs%20BP%20Controller))
  ;[0.15 0.15 0.15 0.5] 从FP过渡到Build，并切换控制以及重设输入映射
  (bind _returnvalue (Actor|GetActorOfClass "/Game/Bluprints/Characters/Player/BP_Character_Build.BP_Character_Build_C"))
  (Game|Player|SetViewTargetwithBlend _as_bp_controller _returnvalue 2.5 "VTBlend_Cubic" 0.0 false)
  (Utilities|FlowControl|Delay 3.0)
  (Default|SwitchPossess _as_bp_controller (Pawn|GetControlledPawn _as_bp_controller) _returnvalue "/Game/Input/FP/IMC_FP.IMC_FP" "/Game/Input/Build/IMC_Build.IMC_Build")
  (Default|SetSpringArmLen _returnvalue 3.5e+03)
  (Default|SetBuildMeshes _returnvalue "/Game/MeshAssets/BuildChunks/Bridge/MS_Build_Bridge_0.MS_Build_Bridge_0" "/Game/MeshAssets/BuildChunks/Bridge/MS_Build_Bridge_1.MS_Build_Bridge_1" "/Game/MeshAssets/BuildChunks/Bridge/MS_Build_Bridge_2.MS_Build_Bridge_2" "/Game/MeshAssets/BuildChunks/Bridge/MS_Build_Bridge_3.MS_Build_Bridge_3" "/Game/MeshAssets/BuildChunks/Bridge/MS_Build_Bridge_4.MS_Build_Bridge_4" "/Game/MeshAssets/BuildChunks/Bridge/MS_Build_Bridge_0.MS_Build_Bridge_0" "/Game/MeshAssets/BuildChunks/Bridge/MS_Build_Bridge_1.MS_Build_Bridge_1")
  (Variables|Default|SetSubLevelState "NewEnumerator1"))

(event EventBeginPlay
  (|CallParentFunction))

(fn ConstructionScript)