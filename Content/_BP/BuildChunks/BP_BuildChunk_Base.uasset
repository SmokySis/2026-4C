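; Base Blueprint for build chunks, handling the material shown on each chunk's static mesh components.
; When InScene is set, the construction script applies MI_BuildChunk to material slot 0 of every static mesh under the root.
; The ChangeMat event applies a supplied material to the same slot on those meshes, then makes the StaticMesh component ignore all collision channels.
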(event Custom|Change%20Mat
  (params (Material :type Material%20Interface%20Object%20Reference))
  (Utilities|FlowControl|Sequence
    (:then_0
      (for _array_element (Components|GetChildrenComponents (Variables|Default|GetDefaultSceneRoot) true)
        (bind _asstatic_mesh_component (Utilities|Casting|CastToStaticMeshComponent _array_element))
        (Rendering|Material|SetMaterial _asstatic_mesh_component 0 Material)))
    (:then_1
      (Collision|SetCollisionResponsetoAllChannels (Variables|Default|GetStaticMesh) "ECR_Ignore"))))

(fn ConstructionScript
  (if (Variables|Default|GetInScene)
    (for _array_element (Components|GetChildrenComponents (Variables|Default|GetDefaultSceneRoot) true)
      (bind _asstatic_mesh_component (Utilities|Casting|CastToStaticMeshComponent _array_element))
      (Rendering|Material|SetMaterial _asstatic_mesh_component 0 "/Game/Materials/MI_BuildChunk.MI_BuildChunk"))))