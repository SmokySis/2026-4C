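; Bridge scene actor that plays short teaching camera shots when the player overlaps its Dun, Plane, Gong or Body trigger components.
; Each overlap shows a WBP_E widget, waits FakeETime, activates that part's camera and blends the view to this actor.
; A part-specific teaching widget shows for five seconds before the view blends back to the pawn.
; The Dun trigger also opens WBP_Pass afterwards.
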(event OnComponentBeginOverlap(Dun)
  (params (OverlappedComponent :type Primitive%20Component%20Object%20Reference) (OtherActor :type Actor%20Object%20Reference) (OtherComp :type Primitive%20Component%20Object%20Reference) (OtherBodyIndex :type Integer) (bFromSweep :type Boolean) (SweepResult :type Hit%20Result%20Structure%20%28by%20ref%29))
  (if (Actor|ActorHasTag OtherActor "player")
    (Widget|SetVisibility (Variables|Default|GetWidget) "Visible")
    (Utilities|FlowControl|Delay (Variables|Default|GetFake%20E%20Time))
    (for _array_element (Variables|Default|GetCam%20Array)
      (Components|Activation|SetActive _array_element false false))
    (Components|Activation|SetActive (Variables|Default|GetDun%20Cam) true false)
    (Game|Player|SetViewTargetwithBlend (Game|GetPlayerController 0) self 2.0 "VTBlend_Cubic" 0.0 false)
    (Utilities|FlowControl|Sequence
      (:then_0
        (Utilities|FlowControl|Delay 5.0)
        (Game|Player|SetViewTargetwithBlend (Game|GetPlayerController 0) (Game|Player|GetPlayerPawn 0) 2.0 "VTBlend_Cubic" 0.0 false)
        (Widget|RemovefromParent (Variables|Default|GetTeach%20UI))
        (Utilities|FlowControl|Delay 1.0)
        (bind _returnvalue (UserInterface|CreateWidget "/Game/UI/WBP_Pass.WBP_Pass_C"))
        (UserInterface|Viewport|AddtoViewport _returnvalue 0))
      (:then_1
        (bind _returnvalue_2 (UserInterface|CreateWidget "/Game/UI/Feature/WBP_F_2_2.WBP_F_2_2_C"))
        (bind _output_get (Variables|Default|SetTeach%20UI _returnvalue_2))
        (UserInterface|Viewport|AddtoViewport _output_get 0))
      (:then_2
        (Widget|SetVisibility (Variables|Default|GetWidget) "Hidden")))))

(event OnComponentBeginOverlap(Plane)
  (params (OverlappedComponent :type Primitive%20Component%20Object%20Reference) (OtherActor :type Actor%20Object%20Reference) (OtherComp :type Primitive%20Component%20Object%20Reference) (OtherBodyIndex :type Integer) (bFromSweep :type Boolean) (SweepResult :type Hit%20Result%20Structure%20%28by%20ref%29))
  (if (Actor|ActorHasTag OtherActor "player")
    (Widget|SetVisibility (Variables|Default|GetWidget) "Visible")
    (Utilities|FlowControl|Delay (Variables|Default|GetFake%20E%20Time))
    (for _array_element (Variables|Default|GetCam%20Array)
      (Components|Activation|SetActive _array_element false false))
    (Components|Activation|SetActive (Variables|Default|GetPlane%20Cam) true false)
    (Game|Player|SetViewTargetwithBlend (Game|GetPlayerController 0) self 2.0 "VTBlend_Cubic" 0.0 false)
    (Utilities|FlowControl|Sequence
      (:then_0
        (Utilities|FlowControl|Delay 5.0)
        (Game|Player|SetViewTargetwithBlend (Game|GetPlayerController 0) (Game|Player|GetPlayerPawn 0) 2.0 "VTBlend_Cubic" 0.0 false)
        (Widget|RemovefromParent (Variables|Default|GetTeach%20UI)))
      (:then_1
        (bind _returnvalue (UserInterface|CreateWidget "/Game/UI/Feature/WBP_F_2_3.WBP_F_2_3_C"))
        (bind _output_get (Variables|Default|SetTeach%20UI _returnvalue))
        (UserInterface|Viewport|AddtoViewport _output_get 0))
      (:then_2
        (Widget|SetVisibility (Variables|Default|GetWidget) "Hidden")))))

(event OnComponentBeginOverlap(Gong)
  (params (OverlappedComponent :type Primitive%20Component%20Object%20Reference) (OtherActor :type Actor%20Object%20Reference) (OtherComp :type Primitive%20Component%20Object%20Reference) (OtherBodyIndex :type Integer) (bFromSweep :type Boolean) (SweepResult :type Hit%20Result%20Structure%20%28by%20ref%29))
  (if (Actor|ActorHasTag OtherActor "player")
    (Widget|SetVisibility (Variables|Default|GetWidget) "Visible")
    (Utilities|FlowControl|Delay (Variables|Default|GetFake%20E%20Time))
    (for _array_element (Variables|Default|GetCam%20Array)
      (Components|Activation|SetActive _array_element false false))
    (Components|Activation|SetActive (Variables|Default|GetGong%20Cam) true false)
    (Game|Player|SetViewTargetwithBlend (Game|GetPlayerController 0) self 2.0 "VTBlend_Cubic" 0.0 false)
    (Utilities|FlowControl|Sequence
      (:then_0
        (Utilities|FlowControl|Delay 5.0)
        (Game|Player|SetViewTargetwithBlend (Game|GetPlayerController 0) (Game|Player|GetPlayerPawn 0) 2.0 "VTBlend_Cubic" 0.0 false)
        (Widget|RemovefromParent (Variables|Default|GetTeach%20UI)))
      (:then_1
        (bind _returnvalue (UserInterface|CreateWidget "/Game/UI/Feature/WBP_F_2_4.WBP_F_2_4_C"))
        (bind _output_get (Variables|Default|SetTeach%20UI _returnvalue))
        (UserInterface|Viewport|AddtoViewport _output_get 0))
      (:then_2
        (Widget|SetVisibility (Variables|Default|GetWidget) "Hidden")))))

(event OnComponentBeginOverlap(Body)
  (params (OverlappedComponent :type Primitive%20Component%20Object%20Reference) (OtherActor :type Actor%20Object%20Reference) (OtherComp :type Primitive%20Component%20Object%20Reference) (OtherBodyIndex :type Integer) (bFromSweep :type Boolean) (SweepResult :type Hit%20Result%20Structure%20%28by%20ref%29))
  (if (Actor|ActorHasTag OtherActor "player")
    (Widget|SetVisibility (Variables|Default|GetWidget) "Visible")
    (Utilities|FlowControl|Delay (Variables|Default|GetFake%20E%20Time))
    (for _array_element (Variables|Default|GetCam%20Array)
      (Components|Activation|SetActive _array_element false false))
    (Components|Activation|SetActive (Variables|Default|GetBody%20Cam) true false)
    (Game|Player|SetViewTargetwithBlend (Game|GetPlayerController 0) self 2.0 "VTBlend_Cubic" 0.0 false)
    (Utilities|FlowControl|Sequence
      (:then_0
        (Utilities|FlowControl|Delay 5.0)
        (Game|Player|SetViewTargetwithBlend (Game|GetPlayerController 0) (Game|Player|GetPlayerPawn 0) 2.0 "VTBlend_Cubic" 0.0 false)
        (Widget|RemovefromParent (Variables|Default|GetTeach%20UI)))
      (:then_1
        (bind _returnvalue (UserInterface|CreateWidget "/Game/UI/Feature/WBP_F_2_1.WBP_F_2_1_C"))
        (bind _output_get (Variables|Default|SetTeach%20UI _returnvalue))
        (UserInterface|Viewport|AddtoViewport _output_get 0))
      (:then_2
        (Widget|SetVisibility (Variables|Default|GetWidget) "Hidden")))))

(event EventBeginPlay
  (bind _cam_array (Variables|Default|GetCam%20Array))
  (bind _returnvalue (UserInterface|CreateWidget "/Game/UI/WBP_E.WBP_E_C"))
  (bind _output_get (Variables|Default|SetWidget _returnvalue))
  (Widget|SetVisibility _output_get "Hidden")
  (UserInterface|Viewport|AddtoViewport _output_get 0)
  (Utilities|Array|Add _cam_array (Variables|Default|GetPlane%20Cam))
  (Utilities|Array|Add _cam_array (Variables|Default|GetGong%20Cam))
  (Utilities|Array|Add _cam_array (Variables|Default|GetBody%20Cam))
  (Utilities|Array|Add _cam_array (Variables|Default|GetDun%20Cam)))

(fn ConstructionScript)