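; BP_WoodBridge1 is a wood bridge piece in what appears to be a SunMao (mortise-and-tenon) assembly puzzle.
; When its Box begins overlapping an actor of exact class BP_WoodBridge0 whose IsOver flag is set, it sets its own IsOver.
; It then finds BP_JointControll in the level and calls CheckIsOver, so completion chains from the preceding piece to the controller.
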(event OnComponentBeginOverlap(Box)
  (params (OverlappedComponent :type Primitive%20Component%20Object%20Reference) (OtherActor :type Actor%20Object%20Reference) (OtherComp :type Primitive%20Component%20Object%20Reference) (OtherBodyIndex :type Integer) (bFromSweep :type Boolean) (SweepResult :type Hit%20Result%20Structure%20%28by%20ref%29))
  (if (== (Utilities|GetClass OtherActor) "/Game/_BP/SunMao/WoodBridge/BP_WoodBridge0.BP_WoodBridge0_C")
    (bind _asbp_sun_mao_base (Utilities|Casting|CastToBP_SunMao_Base OtherActor))
    (if (Variables|/Game/_BP/SunMao/BP_SunMao_Base.BP_SunMao_Base_C|GetIsOver? _asbp_sun_mao_base)
      (Variables|Default|SetIsOver? true)
      (bind _returnvalue (Actor|GetActorOfClass "/Game/Bluprints/Characters/Player/BP_JointControll.BP_JointControll_C"))
      (Default|CheckIsOver? _returnvalue))))

(event EventBeginPlay
  (|CallParentFunction) ; 此节点被禁用，将不会被调用。\n从引脚连出引线来编译功能。
)

(event Collision|EventActorBeginOverlap
  (params (OtherActor :type Actor%20Object%20Reference))
  (|CallParentFunction OtherActor) ; 此节点被禁用，将不会被调用。\n从引脚连出引线来编译功能。
)

(event EventTick
  (params (DeltaSeconds :type Float%20%28single-precision%29))
  (|CallParentFunction DeltaSeconds) ; 此节点被禁用，将不会被调用。\n从引脚连出引线来编译功能。
)

(fn ConstructionScript
  (|CallParentFunction))