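; BP_Boat05 is a boat actor that travels along the spline of a referenced SplineToFollow actor, starting on BeginPlay.
; A timeline, with its play rate set to the inverse of TimeToComplete, drives a 0-to-spline-length lerp for the distance along the path.
; Each update sets the boat's world location and rotation from that point, adding a 90-degree yaw offset.
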(event Custom|MoveBoat
  (bind _splinetofollow (Variables|Default|GetSplineToFollow))
  (bind _spline (Variables|/Game/chinesewoodenboat/Blueprint/BP_SplinePath.BP_SplinePath_C|GetSpline _splinetofollow))
  (Components|Timeline|SetPlayRate (Variables|Default|GetT_Move) (/ 1.0 (Variables|Default|GetTimeToComplete)))
  (bind _movetrack (Timeline|T_Move Play)
    (:Update
      (Transformation|SetActorLocationAndRotation (Spline|GetLocationatDistanceAlongSpline _spline (Math|Float|Lerp 0.0 (Spline|GetSplineLength _spline) _movetrack) "World") (Math|Rotator|MakeRotator (.roll (Spline|GetRotationatDistanceAlongSpline _spline (Math|Float|Lerp 0.0 (Spline|GetSplineLength _spline) _movetrack) "World")) (.pitch (Spline|GetRotationatDistanceAlongSpline _spline (Math|Float|Lerp 0.0 (Spline|GetSplineLength _spline) _movetrack) "World")) (+ (.yaw (Spline|GetRotationatDistanceAlongSpline _spline (Math|Float|Lerp 0.0 (Spline|GetSplineLength _spline) _movetrack) "World")) 9e+01))))))

(event EventBeginPlay
  (CallFunction|MoveBoat))

(fn ConstructionScript)