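; BP_InteractComp drives NPC dialogue, showing one line each time PlayDialogue is called.
; The first call creates a WBP_Dialogue widget with the NPC name and line; later calls update its text.
; Each data table row supplies the next row name, table and end flag, chaining lines across tables.
; Once a row flags the end, the following call removes and clears the widget.
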(event Custom|PlayDialogue
  (if (Variables|Default|GetEndDialogue?)
    (Widget|RemovefromParent (Variables|Default|GetDialogueUI))
    (Variables|Default|SetEndDialogue? false)
    (Variables|Default|SetDialogueUI 0)
    (else
      (Utilities|IsValid (Variables|Default|GetDialogueUI)
        (:Is%20Valid
          (bind _returnvalue (Utilities|GetDataTableRow (Variables|Default|GetData%20Table) (Variables|Default|GetRow%20Name))
            (:then
              (Default|更新文本 (Variables|Default|GetDialogueUI) (.dialogue (Utilities|Struct|BreakDialogues _returnvalue)))
              (Variables|Default|SetRow%20Name (.row (Utilities|Struct|BreakDialogues _returnvalue)))
              (Variables|Default|SetData%20Table (.datatable (Utilities|Struct|BreakDialogues _returnvalue)))
              (Variables|Default|SetEndDialogue? (.EndDialogue? (Utilities|Struct|BreakDialogues _returnvalue))))))
        (:Is%20Not%20Valid
          (bind _returnvalue_2 (Utilities|GetDataTableRow (Variables|Default|GetData%20Table) (Variables|Default|GetRow%20Name))
            (:then
              (bind _returnvalue_3 (UserInterface|CreateWidget "/Game/UI/WBP_Dialogue.WBP_Dialogue_C" 0 (Utilities|Text|ToText(Name) (Variables|Default|GetNPCName)) (.dialogue (Utilities|Struct|BreakDialogues _returnvalue_2))))
              (bind _output_get (Variables|Default|SetDialogueUI _returnvalue_3))
              (UserInterface|Viewport|AddtoViewport _output_get 0)
              (Variables|Default|SetRow%20Name (.row (Utilities|Struct|BreakDialogues _returnvalue_2)))
              (Variables|Default|SetData%20Table (.datatable (Utilities|Struct|BreakDialogues _returnvalue_2)))
              (Variables|Default|SetEndDialogue? (.EndDialogue? (Utilities|Struct|BreakDialogues _returnvalue_2))))))))))